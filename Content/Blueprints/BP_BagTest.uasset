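; BP_BagTest is a bag actor that rides a conveyor spline until its assigned AI character collects it.
; Hitting a BP_ConveyorBelt flags it, and a later hit after grabber release starts a spline-following timeline, offset by the scaled closest spline input key.
; When the character whose BagToCollectRef matches overlaps it, the bag copies its mesh and scale onto that character, sends them to their collection point and destroys itself.
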(event `self.ReceiveBeginPlay`
  (bind _outactors (`GameplayStatics.GetAllActorsOfClass` "/Game/Blueprints/Conveyor/BP_Spline.BP_Spline_C"))
  (set `self.SplineRef` (`|GetArrayItem` _outactors)))

(event `MoveThisActor`
  (params (NewStartTime :type "Float (double-precision)"))
  (bind _spline (`/Game/Blueprints/Conveyor/BP_Spline.Spline` (`self.SplineRef`)))
  (`TimelineComponent.SetNewTime` (`self.MovementTimeline`) NewStartTime)
  (bind (_direction _movementalpha) (`Timeline|MovementTimeline` :`NewTime` NewStartTime)
    (:`Update`
      (bind _returnvalue (`KismetMathLibrary.Lerp` 0.0 (`SplineComponent.GetSplineLength` _spline) _movementalpha))
      (`self.K2_SetActorLocationAndRotation` (`SplineComponent.GetLocationAtDistanceAlongSpline` _spline _returnvalue "World") (`SplineComponent.GetRotationAtDistanceAlongSpline` _spline _returnvalue "World")))))

(event `self.MeshComp.OnComponentHit`
  (params (HitComponent :type "PrimitiveComponent Object Reference") (OtherActor :type "Actor Object Reference") (OtherComp :type "PrimitiveComponent Object Reference") (NormalImpulse :type "Vector Structure") (Hit :type "HitResult Structure (by ref)"))
  (if (`self.IsOverlappingSpline`)
    (if (and (`self.GrabberHasBeenReleased`) (not (`self.TimelineHasStarted`)))
      (set `self.TimelineHasStarted` true)
      (`self.MoveThisActor` (* (`SplineComponent.FindInputKeyClosestToWorldLocation` (`/Game/Blueprints/Conveyor/BP_Spline.Spline` (`self.SplineRef`)) (`self.K2_GetActorLocation`)) 0.08)))
    (else
      (cast `/Game/Blueprints/Conveyor/BP_ConveyorBelt` OtherActor)
      (set `self.IsOverlappingSpline` true))))

(event `self.BoxCollision.OnComponentBeginOverlap`
  (params (OverlappedComponent :type "PrimitiveComponent Object Reference") (OtherActor :type "Actor Object Reference") (OtherComp :type "PrimitiveComponent Object Reference") (OtherBodyIndex :type Integer) (bFromSweep :type Boolean) (SweepResult :type "HitResult Structure (by ref)"))
  (bind _meshcomp (`self.MeshComp`))
  (bind _asbp_aicharacter (cast `/Game/Blueprints/AI/BP_AICharacter` OtherActor))
  (if (== self (`/Game/Blueprints/AI/BP_AICharacter.BagToCollectRef` _asbp_aicharacter))
    (`TimelineComponent.Stop` (`self.MovementTimeline`))
    (bind _bagcollectedmesh (`/Game/Blueprints/AI/BP_AICharacter.BagCollectedMesh` _asbp_aicharacter))
    (`StaticMeshComponent.SetStaticMesh` _bagcollectedmesh (`StaticMeshComponent.StaticMesh` _meshcomp))
    (`SceneComponent.SetWorldScale3D` _bagcollectedmesh (`SceneComponent.K2_GetComponentScale` _meshcomp))
    (`AIBlueprintHelperLibrary.SimpleMoveToLocation` (`Pawn.GetController` _asbp_aicharacter) (`SceneComponent.K2_GetComponentLocation` (`ConveyorCollectionPointActor.CollectedPointArrow` (`/Game/Blueprints/AI/BP_AICharacter.CollectionPointRef` _asbp_aicharacter))))
    (`self.K2_DestroyActor`)))

(fn `UserConstructionScript`)