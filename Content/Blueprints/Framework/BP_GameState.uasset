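; Game state that drives an endless bag and AI spawn loop, speeding it up over time.
; BeginPlay caches collection, spawn and exit points, then finds the TP_BagSpawn target point by display name.
; A looping delay chain spawns a randomly offset bag, reserves an unassigned collection point, and spawns an AI at a random spawn point with both references.
; Tick periodically shortens the delay down to a floor.
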(event `self.ReceiveTick`
  (params (DeltaSeconds :type "Float (single-precision)"))
  (bind _bagspawndelay (`self.BagSpawnDelay`))
  (bind _output_get (set `self.TimeSinceLastSpawn` (+ (`self.TimeSinceLastSpawn`) DeltaSeconds)))
  (if (and (> _output_get (`self.TimeBetweenSpawnSpeedIncrease`)) (> _bagspawndelay 0.5))
    (set `self.BagSpawnDelay` (- _bagspawndelay 0.5))
    (set `self.TimeSinceLastSpawn` 0.0)))

(event `self.ReceiveBeginPlay`
  (bind _returnvalue (`KismetMathLibrary.RandomFloatInRange` -50.0 50.0))
  (bind _returnvalue_2 (`KismetMathLibrary.RandomFloatInRange` -50.0 50.0))
  (bind (_bagspawnlocation_x _bagspawnlocation_y _bagspawnlocation_z) (`KismetMathLibrary.BreakVector` (`self.BagSpawnLocation`)))
  (bind _spawnpointlocations (`self.SpawnPointLocations`))
  (bind _outactors (`GameplayStatics.GetAllActorsOfClass` "/Game/Blueprints/BP_CollectionPoint.BP_CollectionPoint_C"))
  (for _array_element _outactors
    (`KismetArrayLibrary.Array_Add` (`self.CollectionPoints`) _array_element))
  (bind _outactors_2 (`GameplayStatics.GetAllActorsOfClass` "/Game/Blueprints/AI/BP_AISpawnPoint.BP_AISpawnPoint_C"))
  (for _array_element_2 _outactors_2
    (`KismetArrayLibrary.Array_Add` (`self.SpawnPointLocations`) (`SceneComponent.K2_GetComponentLocation` (`SpawnDestroyAIActor.ArrowComp` _array_element_2))))
  (bind _outactors_3 (`GameplayStatics.GetAllActorsOfClass` "/Game/Blueprints/AI/BP_AIExit.BP_AIExit_C"))
  (for _array_element_3 _outactors_3
    (`KismetArrayLibrary.Array_Add` (`self.ExitPointLocations`) (`SceneComponent.K2_GetComponentLocation` (`SpawnDestroyAIActor.ArrowComp` _array_element_3))))
  (bind _outactors_4 (`GameplayStatics.GetAllActorsOfClass` "/Script/Engine.TargetPoint"))
  (for _array_element_4 _outactors_4
    (if (`KismetStringLibrary.EqualEqual_StrStr` (`KismetSystemLibrary.GetDisplayName` _array_element_4) "TP_BagSpawn")
      (set `self.BagSpawnLocation` (`self.K2_GetActorLocation` _array_element_4))
      (bind _returnvalue_3 (`|SpawnActorFromClass` "/Game/Blueprints/BP_BagTest.BP_BagTest_C" (`KismetMathLibrary.MakeTransform` (`KismetMathLibrary.MakeVector` (+ _bagspawnlocation_x _returnvalue) (+ _bagspawnlocation_y _returnvalue) _bagspawnlocation_z) (`KismetMathLibrary.MakeRotator` _returnvalue_2 _returnvalue_2 _returnvalue_2) (1.0 1.0 0.5)) "AdjustIfPossibleButAlwaysSpawn" "OverrideRootScale" null null :!label _label))
      (`KismetSystemLibrary.Delay` (/ (`self.BagSpawnDelay`) 2.0))
      (for _array_element_5 (`self.CollectionPoints`)
        (if (not (`ConveyorCollectionPointActor.GetHasBeenAssigned` _array_element_5))
          (`ConveyorCollectionPointActor.SetHasBeenAssigned` _array_element_5 true)
          (break)))
      (`|SpawnActorFromClass` "/Game/Blueprints/AI/BP_AICharacter.BP_AICharacter_C" (`KismetMathLibrary.MakeTransform` (`|GetArrayItem` _spawnpointlocations (`KismetMathLibrary.RandomIntegerInRange` 0 (- (`KismetArrayLibrary.Array_Length` _spawnpointlocations) 1)))) "AdjustIfPossibleButAlwaysSpawn" "OverrideRootScale" null _returnvalue_3 _array_element_5 null)
      (`KismetSystemLibrary.Delay` (/ (`self.BagSpawnDelay`) 2.0))
      (goto _label))))

(fn `UserConstructionScript`)