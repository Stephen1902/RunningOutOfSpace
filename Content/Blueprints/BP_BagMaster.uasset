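; BP_BagMaster is a bag actor that rides a conveyor belt along the level's BP_Spline.
; A hit on BP_ConveyorBelt flags it; a later hit after grabber release starts it once and registers it with BP_GameState.
; A timeline drives position and rotation along the spline, starting from the closest input key scaled to timeline time.
; Character pickup logic exists but is disconnected, and the box overlap does nothing.
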(event `self.ReceiveBeginPlay`
  (bind _outactors (`GameplayStatics.GetAllActorsOfClass` "/Game/Conveyor/BP_Spline.BP_Spline_C"))
  (set `self.SplineRef` (`|GetArrayItem` _outactors))
  (bind _asbp_game_state (cast `/Game/Blueprints/Framework/BP_GameState` (`GameplayStatics.GetGameState`)))
  (set `self.GameStateRef` _asbp_game_state))

(event `MoveThisActor`
  (params (NewStartTime :type "Float (double-precision)"))
  (bind _spline (`/Game/Conveyor/BP_Spline.Spline` (`self.SplineRef`)))
  (`TimelineComponent.SetNewTime` (`self.MovementTimeline`) NewStartTime)
  (bind (_direction _movementalpha) (`Timeline|MovementTimeline` :`NewTime` NewStartTime)
    (:`Update`
      (bind _returnvalue (`KismetMathLibrary.Lerp` 0.0 (`SplineComponent.GetSplineLength` _spline) _movementalpha))
      (`self.K2_SetActorLocationAndRotation` (`SplineComponent.GetLocationAtDistanceAlongSpline` _spline _returnvalue "World") (`SplineComponent.GetRotationAtDistanceAlongSpline` _spline _returnvalue "World")))))

(event `self.StaticMesh.OnComponentHit`
  (params (HitComponent :type "PrimitiveComponent Object Reference") (OtherActor :type "Actor Object Reference") (OtherComp :type "PrimitiveComponent Object Reference") (NormalImpulse :type "Vector Structure") (Hit :type "HitResult Structure (by ref)"))
  (if (`self.IsOverlappingSpline`)
    (if (and (`self.GrabberHasBeenReleased`) (not (`self.TimelineHasStarted`)))
      (set `self.TimelineHasStarted` true)
      (`self.MoveThisActor` (* (`SplineComponent.FindInputKeyClosestToWorldLocation` (`/Game/Conveyor/BP_Spline.Spline` (`self.SplineRef`)) (`self.K2_GetActorLocation`)) 0.08))
      (`/Game/Blueprints/Framework/BP_GameState.AddBagToArray` (`self.GameStateRef`) self))
    (else
      (cast `/Game/Conveyor/BP_ConveyorBelt` OtherActor)
      (set `self.IsOverlappingSpline` true))))

(event `self.Box.OnComponentBeginOverlap`
  (params (OverlappedComponent :type "PrimitiveComponent Object Reference") (OtherActor :type "Actor Object Reference") (OtherComp :type "PrimitiveComponent Object Reference") (OtherBodyIndex :type Integer) (bFromSweep :type Boolean) (SweepResult :type "HitResult Structure (by ref)")))

(fn `UserConstructionScript`)